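; A placeable item Blueprint whose skeletal mesh may play a one-shot animation when something enters its trigger box.
; On BeginPlay it assigns the configured mesh and rolls a random chance of roughly one in ten to become animatable.
; An animatable item plays its configured animation on the first box overlap, with no filter on the overlapping actor, and a flag blocks any replay.
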(event OnComponentBeginOverlap(Box)
  (params (OverlappedComponent :type Primitive%20Component%20Object%20Reference) (OtherActor :type Actor%20Object%20Reference) (OtherComp :type Primitive%20Component%20Object%20Reference) (OtherBodyIndex :type Integer) (bFromSweep :type Boolean) (SweepResult :type Hit%20Result%20Structure%20%28by%20ref%29))
  (if (and (Variables|Default|GetCanAnimate) (not (Variables|Default|GetAnimateFinished)))
    (Variables|Default|SetAnimateFinished true)
    (Components|Animation|PlayAnimation (Variables|Default|GetSkeletalMesh) (Variables|Default|Getanimation) false)))

(event EventBeginPlay
  (Class|SkinnedMeshComponent|SetSkeletalMesh (Variables|Default|GetSkeletalMesh) (Variables|Default|GetMeshModel) true)
  (if (<= (Math|Random|RandomInteger 100) 10)
    (Variables|Default|SetCanAnimate true)
    (else
      (Variables|Default|SetCanAnimate false))))

(fn ConstructionScript)